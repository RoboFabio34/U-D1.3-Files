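; Jump selector gimmick that catches the dash player pawn and launches it in a direction chosen by Jump, Action or Duck input.
; Overlap freezes and snaps the pawn, moves input to the selector and starts a timeout timeline that forces a penalty release.
; Release rotates the model by timeline, launches the pawn, then plays right/wrong sound by comparing selector states.
; Construction script sets the selector's state colour through a material UV parameter.
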(event Custom|Timer%20TO%20FUCK%20YOU
  (Timeline|TL-FUCK%20YOU PlayFromStart
    (:Finished
      (Audio|Components|Audio|Stop (Variables|Default|GetJumpSelector_Cue))
      (CallFunction|ReleaseJump 9e+01 true))))

(event Custom|No%20longer%20fuck%20you
  (Timeline|TL-FUCK%20YOU Stop
    (:Finished
      (Audio|Components|Audio|Stop (Variables|Default|GetJumpSelector_Cue))
      (CallFunction|ReleaseJump 9e+01 true))))

(event EventBeginPlay
  (Utilities|FlowControl|DoOnce false
    (:Completed
      (Audio|Components|Audio|Stop (Variables|Default|GetJumpSelector_Cue)))))

(event Input|ActionEvents|InputActionJump
  (params (Key :type Key%20Structure :default "None"))
  (:Pressed
    (Variables|/Game/DashEngine/System/DashPlayerPawn.DashPlayerPawn_C|SetJumpSelectorState (CallFunction|GetDashPlayerPawn) 0)
    (CallFunction|ReleaseJump -9e+01 false)))

(event Input|ActionEvents|InputActionAction
  (params (Key :type Key%20Structure :default "None"))
  (:Pressed
    (Variables|/Game/DashEngine/System/DashPlayerPawn.DashPlayerPawn_C|SetJumpSelectorState (CallFunction|GetDashPlayerPawn) 1)
    (CallFunction|ReleaseJump 0.0 false)))

(event Input|ActionEvents|InputActionDuck
  (params (Key :type Key%20Structure :default "None"))
  (:Pressed
    (CallFunction|ReleaseJump 9e+01 false)))

(fn ConstructionScript
  (bind _returnvalue (Rendering|Material|CreateDynamicMaterialInstance (Variables|Default|Getcmn_obj_jselector_HD_model) 2 "/Game/DashEngine/Objects/JumpSelector/Textures/M_Metal_JumpSelector02_Inst.M_Metal_JumpSelector02_Inst" "None" :!class /Script/Engine.PrimitiveComponent))
  (Rendering|Material|SetVectorParameterValue _returnvalue "Uv control" (Utilities|Select :Index (Variables|Default|GetJumpSelector%20State) :NewEnumerator0 "" :NewEnumerator2 "(R=0.000000,G=0.500000,B=0.000000,A=1.000000)" :NewEnumerator1 "(R=0.500000,G=0.000000,B=0.000000,A=1.000000)" :NewEnumerator3 "(R=0.500000,G=0.500000,B=0.000000,A=1.000000)") :!class /Script/Engine.MaterialInstanceDynamic))

(event Custom|Release%20Jump
  (params (Rotation%20Look%20into :type Float%20%28single-precision%29) (FUCK%20YOU :type Boolean))
  (bind _playercontroller (CallFunction|GetDashPlayerController))
  (bind _pawn (Variables|SwingPole|Runtime|GetPawn))
  (CallFunction|NoLongerFuckYou)
  (Components|Animation|PlayAnimation (Variables|Default|Getcmn_obj_jselector_HD_model) "/Game/DashEngine/Objects/JumpSelector/Model/JumpSelectorAnim.JumpSelectorAnim" false)
  (Variables|Default|SetInternal%20Rot%20before%20launch (Variables|/Script/Engine.SceneComponent|GetRelativeRotation (Variables|Default|Getcmn_obj_jselector_HD_model)))
  (bind _alpha (Timeline|TL_Move%20Selector%20Up PlayFromStart)
    (:Update
      (Transformation|SetRelativeRotation (Variables|Default|Getcmn_obj_jselector_HD_model) (Math|Rotator|Lerp(Rotator) (Variables|Default|GetInternal%20Rot%20before%20launch) (Math|Rotator|MakeRotator Rotation%20Look%20into 0.0 -9e+01) _alpha) false false))
    (:Finished
      (Audio|Components|Audio|Stop (Variables|Default|GetJumpSelector_Cue))
      (Variables|SwingPole|Runtime|SetReleased? true)
      (Pawn|Components|CharacterMovement|SetMovementMode (Variables|/Script/Engine.Character|GetCharacterMovement (Variables|SwingPole|Runtime|GetPawn)) "MOVE_Falling" 0)
      (Character|LaunchCharacter (Variables|SwingPole|Runtime|GetPawn) (|DetermineLaunchVelocity FUCK%20YOU) true true)
      (Default|ChangeState (Variables|SwingPole|Runtime|GetPawn) "NewEnumerator3" "NewEnumerator52" "NewEnumerator0")
      (Default|ResetUseShield _pawn)
      (Default|ClearHomingTarget _pawn true true)
      (Input|DisableInput self _playercontroller)
      (Input|EnableInput _playercontroller _playercontroller)
      (Variables|/Game/DashEngine/System/DashPlayerPawn.DashPlayerPawn_C|SetOnSwingPole? (Variables|SwingPole|Runtime|GetPawn) false)
      (Utilities|FlowControl|Sequence
        (:then_0
          (Utilities|FlowControl|Delay 0.2)
          (Variables|SwingPole|Runtime|SetReleased? false)
          (CallFunction|ResetCol))
        (:then_1
          (if FUCK%20YOU
            (Audio|PlaySound2D "/Game/DashEngine/Objects/JumpSelector/SFX/0020_objsn_jumpslct_wrong.0020_objsn_jumpslct_wrong" 1.0 1.0 0.0 0 0)
            (elif (== (Variables|Default|GetJumpSelector%20State) (Variables|/Game/DashEngine/System/DashPlayerPawn.DashPlayerPawn_C|GetJumpSelectorState (CallFunction|GetDashPlayerPawn)))
              (Audio|PlaySound2D "/Game/DashEngine/Objects/JumpSelector/SFX/0021_objsn_jumpslct_ok.0021_objsn_jumpslct_ok" 1.0 1.0 0.0 0 0)
              (else
                (Audio|PlaySound2D "/Game/DashEngine/Objects/JumpSelector/SFX/0020_objsn_jumpslct_wrong.0020_objsn_jumpslct_wrong" 1.0 1.0 0.0 0 0)))))))))

(event OnComponentBeginOverlap(Collision)
  (params (OverlappedComponent :type Primitive%20Component%20Object%20Reference) (OtherActor :type Actor%20Object%20Reference) (OtherComp :type Primitive%20Component%20Object%20Reference) (OtherBodyIndex :type Integer) (bFromSweep :type Boolean) (SweepResult :type Hit%20Result%20Structure%20%28by%20ref%29))
  (bind _playercontroller (CallFunction|GetDashPlayerController))
  (Utilities|FlowControl|DoOnce false
    (:Completed
      (if (not (Variables|SwingPole|Runtime|GetReleased?))
        (bind _asdash_player_pawn (Utilities|Casting|CastToDashPlayerPawn OtherActor))
        (Variables|SwingPole|Runtime|SetPawn _asdash_player_pawn)
        (Default|ForceStopRushTrick (Variables|SwingPole|Runtime|GetPawn))
        (Default|StopHomingAttack (Variables|SwingPole|Runtime|GetPawn))
        (Variables|/Game/DashEngine/System/DashPlayerPawn.DashPlayerPawn_C|SetOnSwingPole? (Variables|SwingPole|Runtime|GetPawn) true)
        (Default|ChangeAnimState (Variables|SwingPole|Runtime|GetPawn) "NewEnumerator51")
        (Pawn|Components|CharacterMovement|DisableMovement (Variables|/Script/Engine.Character|GetCharacterMovement (Variables|SwingPole|Runtime|GetPawn)))
        (Transformation|SetActorRotation (Variables|SwingPole|Runtime|GetPawn) (Transformation|GetActorRotation) true)
        (Transformation|SetActorLocation (Variables|SwingPole|Runtime|GetPawn) (Transformation|GetWorldLocation (Variables|Default|GetCollision)) false true)
        (Input|DisableInput (Variables|SwingPole|Runtime|GetPawn) _playercontroller)
        (Input|EnableInput self _playercontroller)
        (Audio|Components|Audio|Play (Variables|Default|GetJumpSelector_Cue) 0.0)
        (CallFunction|TimerTOFUCKYOU)))))

(event Custom|Reset%20Col
  (bind _playercontroller (CallFunction|GetDashPlayerController))
  (Utilities|FlowControl|DoOnce false) ; enters at Reset
)